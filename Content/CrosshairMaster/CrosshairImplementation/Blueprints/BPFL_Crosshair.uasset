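; Blueprint function library for the crosshair system, exposing the level's BP_Crosshair global scale, tint, offset, AA and recoil settings, plus small vector and sRGB helpers.
; Getters use the first BP_Crosshair found, warning on duplicates, and most fall back to defaults without one.
; Scale derives from camera FOV and viewport width against a 1280x720 base.
; Design time is inferred from the absence of a HUD actor, which skips the actor lookup.
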(fn `Abs (Vector2D)`
  (params (in :type "Vector2D Structure"))
  (returns (out :type "Vector2D Structure"))
  (bind (_x _y) (`KismetMathLibrary.BreakVector2D` in))
  ;[1 1 1] Abs for vector2d
  (return (`KismetMathLibrary.MakeVector2D` (`KismetMathLibrary.Abs` _x) (`KismetMathLibrary.Abs` _y))))

(fn `GetCrosshairAAFilterSize`
  (returns (CrosshairAAFilterSize :type "Float (double-precision)"))
  ;[1 1 1] Check crosshair actor is valid
  (if (`KismetSystemLibrary.IsValid` (`self.GetCrosshairActor` null))
    ;[1 1 1] Return AA filter size
    (return (`/Game/CrosshairMaster/CrosshairMigration/Blueprints/BP_Crosshair.AA_Amount_Precentage` (`self.GetCrosshairActor` null)))
    (else
      ;[1 1 1] Return default value
      (return 100.0))))

(fn `GetCrosshairActor`
  (params (Player :type "/Game/Interaction/Blueprints/Pawn/Player/Character_Pawn_FPS Object Reference"))
  (returns (CrosshairActor :type "/Game/CrosshairMaster/CrosshairMigration/Blueprints/BP_Crosshair Object Reference"))
  (locals (AllCrosshairActors :type "Array of /Game/CrosshairMaster/CrosshairMigration/Blueprints/BP_Crosshair Object Reference") (PlayerC :type "/Game/Interaction/Blueprints/Pawn/Player/Character_Pawn_FPS Object Reference"))
  (if (`self.IsDesignTime` null)
    (return null)
    (else
      (bind _outactors (`GameplayStatics.GetAllActorsOfClass` null "/Game/CrosshairMaster/CrosshairMigration/Blueprints/BP_Crosshair.BP_Crosshair_C"))
      (set `local.AllCrosshairActors` _outactors)
      (`|ExecutionSequence`
        (:`then_0`
          ;[1 1 1] Error: No actor exists
          (if (== (`KismetArrayLibrary.Array_Length` (`local.AllCrosshairActors`)) 0)
            (return null)))
        (:`then_1`
          ;[1 1 1] Warning: Multiple Actors
          (if (> (`KismetArrayLibrary.Array_Length` (`local.AllCrosshairActors`)) 1)
            (`KismetSystemLibrary.PrintString` (`local.__WorldContext`) "[Warning] There are two or more crosshairs in the level. Please use a single crosshair. Currently the first crosshair is being used.")))
        (:`then_2`
          ;[1 1 1] Return first actor
          (return (`|GetArrayItem` (`local.AllCrosshairActors`))))))))

(fn `GetCrosshairBaseScreenResolution`
  (returns (BaseResolution :type "Vector2D Structure"))
  (return (1280.0 720.0)))

(fn `GetCrosshairGlobalColor`
  (returns (CrosshairColorAndOpacity :type "LinearColor Structure"))
  (bind _crosshairactor (`self.GetCrosshairActor` null))
  ;[1 1 1] Return crosshair actor's ColorAndOpacity
  (if (`KismetSystemLibrary.IsValid` _crosshairactor)
    (return (`/Game/CrosshairMaster/CrosshairMigration/Blueprints/BP_Crosshair.GlobalTintColor` _crosshairactor))
    (else
      ;[1 1 1] Return default value
      (return (struct :`R` 1.0 :`G` 1.0 :`B` 1.0 :`A` 1.0)))))

(fn `GetCrosshairGlobalOffset`
  (returns (CrosshairOffset :type "Vector2D Structure"))
  ;[1 1 1] Check crosshair actor is valid
  (if (`KismetSystemLibrary.IsValid` (`self.GetCrosshairActor` null))
    ;[1 1 1] Return crosshair actor's Offset
    (return (`/Game/CrosshairMaster/CrosshairMigration/Blueprints/BP_Crosshair.GlobalOffset` (`self.GetCrosshairActor` null)))
    (else
      ;[1 1 1] Return default value
      (return (0.0 0.0)))))

(fn `GetCrosshairRecoilMultiplier`
  (returns (recoilMultplier :type "Float (double-precision)"))
  (bind _crosshairactor (`self.GetCrosshairActor` null))
  ;[1 1 1] Return crosshair actor's recoil multiplier
  (if (`KismetSystemLibrary.IsValid` _crosshairactor)
    (return (`/Game/CrosshairMaster/CrosshairMigration/Blueprints/BP_Crosshair.RecoilMultiplier (pixels)` _crosshairactor))
    (else
      ;[1 1 1] Return default value
      (return 0.0))))

(fn `GetCrosshairScale`
  (returns (ViewportScale :type "Float (double-precision)"))
  (locals (_fov :type "Float (double-precision)"))
  (bind _returnvalue_x (`KismetMathLibrary.BreakVector2D` (`WidgetLayoutLibrary.GetViewportSize` null)))
  (bind _baseresolution_x (`KismetMathLibrary.BreakVector2D` (`self.GetCrosshairBaseScreenResolution` null)))
  ;[1 1 1] Check crosshair actor is valid
  (if (`KismetSystemLibrary.IsValid` (`self.GetCrosshairActor` null))
    (`|ExecutionSequence`
      (:`then_0`
        ;[1 1 1] Set fov
        (set `local._fov` (`PlayerCameraManager.GetFOVAngle` (`GameplayStatics.GetPlayerCameraManager` null))))
      (:`then_1`
        ;[1 1 1] Multiply crosshair actor's scale value
        (return (* (/ (* (`KismetMathLibrary.MultiplyMultiply_FloatFloat` (* (`KismetMathLibrary.DegTan` (* (`local._fov`) 0.5)) 0.5) -1.0) _returnvalue_x 0.5) _baseresolution_x) (`/Game/CrosshairMaster/CrosshairMigration/Blueprints/BP_Crosshair.GlobalScale` (`self.GetCrosshairActor` null))))))
    (else
      ;[1 1 1] Return default value
      (return 1.0))))

(fn `GetSafeViewportSize`
  (returns (ViewportSize :type "Vector2D Structure"))
  ;[1 1 1] Check crosshair actor is valid
  (if (`KismetSystemLibrary.IsValid` (`self.GetCrosshairActor` null))
    ;[1 1 1] Return viewport size
    (return (`WidgetLayoutLibrary.GetViewportSize` null))
    (else
      ;[1 1 1] Return default value
      (return (`self.GetCrosshairBaseScreenResolution` null)))))

(fn `IsDesignTime`
  (returns (isDesignTime :type Boolean))
  ;[1 1 1] If HUD exists, run-time. Otherwise, design-time
  (bind _outactors (`GameplayStatics.GetAllActorsOfClass` null "/Script/Engine.HUD"))
  (return (== (`KismetArrayLibrary.Array_Length` _outactors) 0)))

(fn `LinearColorToSRGB`
  (params (LinearColor_ :type "LinearColor Structure"))
  (returns (SRGB_ :type "LinearColor Structure"))
  (bind (_returnvalue_b _returnvalue_g _returnvalue_r _returnvalue_a) (break `Color` (`KismetMathLibrary.Conv_LinearColorToColor` LinearColor_)))
  (return (make `LinearColor` (/ (`KismetMathLibrary.Conv_ByteToDouble` _returnvalue_r) 255.0) (/ (`KismetMathLibrary.Conv_ByteToDouble` _returnvalue_g) 255.0) (/ (`KismetMathLibrary.Conv_ByteToDouble` _returnvalue_b) 255.0) (/ (`KismetMathLibrary.Conv_ByteToDouble` _returnvalue_a) 255.0))))

(fn `SafeHypotenus`
  (params (`in vector2d` :type "Vector2D Structure"))
  (returns (`return value` :type "Float (double-precision)"))
  (bind (_x _y) (`KismetMathLibrary.BreakVector2D` `in vector2d`))
  ;[1 1 1] If the input vector is 0, return 0.
  (if (and (== _x 0.0) (== _y 0.0))
    (return 0.0)
    (else
      (return (`KismetMathLibrary.Hypotenuse` _x _y)))))

(fn `Truncate (Vector2D)`
  (params (in :type "Vector2D Structure"))
  (returns (out :type "Vector2D Structure"))
  ;[1 1 1] Truncate for vector2d
  (return (`KismetMathLibrary.MakeVector2D` (`KismetMathLibrary.Conv_IntToDouble` (`KismetMathLibrary.FTrunc` in_X)) (`KismetMathLibrary.Conv_IntToDouble` (`KismetMathLibrary.FTrunc` in_Y)))))