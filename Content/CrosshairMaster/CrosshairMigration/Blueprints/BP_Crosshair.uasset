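; BP_Crosshair is an actor that shows a selectable crosshair widget on screen, with a debugger widget toggled by Tab.
; BeginPlay enables player input, builds the crosshair and adds WB_CrosshairDebugger on a top layer.
; Every Tick it polls Index against the active index and, on a change, swaps in the matching widget class from List.
; An invalid Index reverts to the active one and prints an error.
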(event `self.ReceiveBeginPlay`
  (`self.EnableInput` (`GameplayStatics.GetPlayerController` 0))
  (`self.UpdateCrosshairWidget`)
  (bind _returnvalue (`|CreateWidget` "/Game/CrosshairMaster/CrosshairImplementation/UMG/CrosshairDebugger/WB_CrosshairDebugger.WB_CrosshairDebugger_C"))
  (bind _output_get (set `self.debuggerWidget` _returnvalue))
  (`UserWidget.AddToViewport` _output_get 9999))

(event `self.ReceiveTick`
  (params (DeltaSeconds :type "Float (single-precision)"))
  (`self.UpdateCrosshairWidget`))

(event `Key|Tab`
  (params (Key :type "Key Structure"))
  (:`Pressed`
    (if (`|EnumEquality` (`Widget.GetVisibility` (`self.debuggerWidget`)) "Visible")
      (`Widget.SetVisibility` (`self.debuggerWidget`) "Collapsed")
      (else
        (`Widget.SetVisibility` (`self.debuggerWidget`) "Visible")))))

(fn `GetActiveCrosshairIndex`
  (returns (activeCrosshairIndex :type Integer))
  (return (`self.activeCrosshairIndex`)))

(fn `UpdateCrosshairWidget`
  ;[1 1 1] Check index validity
  (if (`KismetArrayLibrary.Array_IsValidIndex` (`self.List`) (`self.Index`))
    ;[1 1 1] Check whether index is changed
    (if (!= (`self.activeCrosshairIndex`) (`self.Index`))
      ;[1 1 1] Apply changed index
      (set `self.activeCrosshairIndex` (`self.Index`))
      ;[1 1 1] Remove current widget
      (if (`KismetSystemLibrary.IsValid` (`self.currentCrosshairWidget`))
        (`Widget.RemoveFromParent` (`self.currentCrosshairWidget`)))
      ;[1 1 1] Create new widget and add to viewport
      (bind _returnvalue (`|CreateWidget` (`|GetArrayItem` (`self.List`) (`self.activeCrosshairIndex`))))
      (bind _output_get (set `self.currentCrosshairWidget` _returnvalue))
      (`UserWidget.AddToViewport` _output_get 0))
    (else
      (set `self.Index` (`self.activeCrosshairIndex`))
      (`KismetSystemLibrary.PrintString` "[Error] The input crosshair index is not a valid index."))))

(fn `UserConstructionScript`)