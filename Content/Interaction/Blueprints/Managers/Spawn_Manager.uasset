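; Spawn manager that places enemy waves near up to two FPS players until game over.
; It caches spawn locations at BeginPlay and refinds players on Tick whenever its list empties.
; SpawnEnemies picks the nearest open location, using sphere traces as a line-of-sight filter when both players exist.
; Enemies spawn at random attached points, register with EnemyManager and close locations reaching their spawn cap.
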(event `self.ReceiveBeginPlay`
  (bind _outactors (`GameplayStatics.GetAllActorsOfClass` "/Game/Interaction/Blueprints/Managers/Spawn/Spawn_Locations.Spawn_Locations_C"))
  (bind _output_get (set `self.SpawnLocations` _outactors)))

(event `self.ReceiveTick`
  (params (DeltaSeconds :type "Float (single-precision)"))
  (if (<= (`KismetArrayLibrary.Array_Length` (`self.Players`)) 0)
    (bind _outactors (`GameplayStatics.GetAllActorsOfClass` "/Game/Interaction/Blueprints/Pawn/Player/Character_Pawn_FPS.Character_Pawn_FPS_C"))
    (bind _output_get (set `self.Players` _outactors))
    (`KismetSystemLibrary.PrintString` "Find Players")))

(fn `PlayerDistances`
  (returns (Location :type "Vector Structure"))
  (bind _players (`self.Players`))
  (bind _returnvalue (`self.K2_GetActorLocation` (`|GetArrayItem` _players 1)))
  (bind _returnvalue_2 (`self.K2_GetActorLocation` (`|GetArrayItem` _players)))
  (if (>= (`KismetMathLibrary.GetPointDistanceToLine` _returnvalue_2 _returnvalue) (`self.PlayerDistanceFocus`))
    (return (`self.K2_GetActorLocation` (`GameplayStatics.GetPlayerCharacter` (`KismetMathLibrary.RandomIntegerInRange` 0 1))))
    (else
      (return (/ (+ _returnvalue_2 _returnvalue) 2)))))

(fn `ResetSpawnManager`
  (`KismetArrayLibrary.Array_Clear` (`self.Players`)))

(fn `SpawnEnemies`
  (params (Enemy :type "Array of Actor Class Reference") (AmountToSpawn :type "Array of Float (double-precision)"))
  (locals (PlayersVisable :type "Map of Integer to Boolean") (SpawnPos :type "/Game/Interaction/Blueprints/Managers/Spawn/Spawn_Locations Object Reference") (IsVisible :type Boolean) (PlayersDistance :type "Map of Integer to Float (double-precision)") (Count :type Integer))
  (bind _leastdistancespawns (`self.LeastDistanceSpawns`))
  (bind _playersdistance (`local.PlayersDistance`))
  (bind _playersvisable (`local.PlayersVisable`))
  (bind _outactors (`self.GetAttachedActors` _leastdistancespawns))
  (set `self.LeastDistanceSpawns` null)
  (set `self.SpawnCount` 0)
  (set `self.LeastDistance` 900000000.0)
  (for _array_element (`self.SpawnLocations`)
    (set `local.SpawnPos` _array_element)
    (bind _asinteraction_game_mode_fps (cast `/Game/Interaction/Interaction_GameMode_FPS` (`GameplayStatics.GetGameMode`)))
    (if (not (`/Game/Interaction/Interaction_GameMode_FPS.IsGameOver` _asinteraction_game_mode_fps))
      (`BlueprintMapLibrary.Map_Clear` (`local.PlayersVisable`))
      (`BlueprintMapLibrary.Map_Clear` (`local.PlayersDistance`))
      (set `local.IsVisible` false)
      (for _array_element_2 (`self.Players`)
        (cast `/Game/Interaction/Blueprints/Pawn/Player/Character_Pawn_FPS` (`GameplayStatics.GetPlayerCharacter` (`/Game/Interaction/Blueprints/Pawn/Player/Character_Pawn_FPS.PlayerID` _array_element_2)))
        (if (`/Game/Interaction/Blueprints/Managers/Spawn/Spawn_Locations.CanSpawn` (`local.SpawnPos`))
          (bind _returnvalue (`self.K2_GetActorLocation` _array_element_2))
          (bind _isnotvisable (`self.SpawnVisable` (`local.SpawnPos`) _returnvalue))
          (`BlueprintMapLibrary.Map_Add` (`local.PlayersVisable`) (`/Game/Interaction/Blueprints/Pawn/Player/Character_Pawn_FPS.PlayerID` _array_element_2) _isnotvisable)
          (`BlueprintMapLibrary.Map_Add` (`local.PlayersDistance`) (`/Game/Interaction/Blueprints/Pawn/Player/Character_Pawn_FPS.PlayerID` _array_element_2) (`KismetMathLibrary.GetPointDistanceToLine` (`self.K2_GetActorLocation` (`local.SpawnPos`)) _returnvalue))))
      (cast `/Game/Interaction/Blueprints/Pawn/Player/Character_Pawn_FPS` (`GameplayStatics.GetPlayerCharacter` 0)
        (:`then`
          (cast `/Game/Interaction/Blueprints/Pawn/Player/Character_Pawn_FPS` (`GameplayStatics.GetPlayerCharacter` 1)
            (:`then`
              (if (and (`BlueprintMapLibrary.Map_Find` _playersvisable) (`BlueprintMapLibrary.Map_Find` _playersvisable 1))
                (if (< (`BlueprintMapLibrary.Map_Find` _playersdistance) (`BlueprintMapLibrary.Map_Find` _playersdistance 1))
                  (if (<= (`BlueprintMapLibrary.Map_Find` (`local.PlayersDistance`)) (`self.LeastDistance`))
                    (set `self.LeastDistance` (`BlueprintMapLibrary.Map_Find` (`local.PlayersDistance`)))
                    (set `self.LeastDistanceSpawns` (`local.SpawnPos`)))
                  (elif (<= (`BlueprintMapLibrary.Map_Find` (`local.PlayersDistance`) 1) (`self.LeastDistance`))
                    (set `self.LeastDistance` (`BlueprintMapLibrary.Map_Find` (`local.PlayersDistance`) 1))
                    (set `self.LeastDistanceSpawns` (`local.SpawnPos`))))))
            (:`CastFailed`
              (if (<= (`BlueprintMapLibrary.Map_Find` (`local.PlayersDistance`)) (`self.LeastDistance`))
                (set `self.LeastDistance` (`BlueprintMapLibrary.Map_Find` (`local.PlayersDistance`)))
                (set `self.LeastDistanceSpawns` (`local.SpawnPos`))))))
        (:`CastFailed`
          (cast `/Game/Interaction/Blueprints/Pawn/Player/Character_Pawn_FPS` (`GameplayStatics.GetPlayerCharacter` 1)
            (:`then`
              (if (<= (`BlueprintMapLibrary.Map_Find` (`local.PlayersDistance`) 1) (`self.LeastDistance`))
                (set `self.LeastDistance` (`BlueprintMapLibrary.Map_Find` (`local.PlayersDistance`) 1))
                (set `self.LeastDistanceSpawns` (`local.SpawnPos`))))
            (:`CastFailed`
              (set `self.LeastDistanceSpawns` null)))))))
  (bind _asinteraction_game_mode_fps_2 (cast `/Game/Interaction/Interaction_GameMode_FPS` (`GameplayStatics.GetGameMode`)))
  (if (not (`/Game/Interaction/Interaction_GameMode_FPS.IsGameOver` _asinteraction_game_mode_fps_2))
    (if (`KismetSystemLibrary.IsValid` (`self.LeastDistanceSpawns`))
      (for (_array_element_3 _array_index) Enemy
        (for _ (range 1 (+ (`KismetMathLibrary.FTrunc` (`|GetArrayItem` AmountToSpawn _array_index)) 1))
          (set `self.SpawnCount` (+ 1 (`self.SpawnCount`)))
          (bind _returnvalue_2 (`|SpawnActorFromClass` _array_element_3 (`self.GetTransform` (`|GetArrayItem` _outactors (`KismetMathLibrary.RandomInteger` (- (`KismetArrayLibrary.Array_Length` _outactors) 1)))) "Undefined" "OverrideRootScale" null null))
          (`/Game/Interaction/Blueprints/Managers/Enemy_Manager.AddEnemy` (`self.EnemyManager`) _returnvalue_2)
          (set `/Game/Interaction/Blueprints/Managers/Spawn/Spawn_Locations.CurrentSpawns` (`KismetMathLibrary.Conv_IntToDouble` (`self.SpawnCount`)) (`self.LeastDistanceSpawns`))))
      (if (>= (`/Game/Interaction/Blueprints/Managers/Spawn/Spawn_Locations.CurrentSpawns` _leastdistancespawns) (`/Game/Interaction/Blueprints/Managers/Spawn/Spawn_Locations.MaxSpawns` _leastdistancespawns))
        (set `/Game/Interaction/Blueprints/Managers/Spawn/Spawn_Locations.CanSpawn` false _leastdistancespawns)))))

(fn `SpawnEnemy`
  (params (Enemy :type "Actor Class Reference"))
  (bind _leastdistancespawns (`self.LeastDistanceSpawns`))
  (bind _outactors (`self.GetAttachedActors` (`self.LeastDistanceSpawns`)))
  (set `self.LeastDistance` 900000000.0)
  (bind _location (`self.PlayerDistances`))
  (for _array_element (`self.SpawnLocations`)
    (bind _isnotvisable (`self.SpawnVisable` _array_element _location))
    (if _isnotvisable
      (bind _returnvalue (`KismetMathLibrary.GetPointDistanceToLine` (`self.K2_GetActorLocation` _array_element) _location))
      (if (<= _returnvalue (`self.LeastDistance`))
        (set `self.LeastDistance` _returnvalue)
        (set `self.LeastDistanceSpawns` _array_element))))
  (`|SpawnActorFromClass` Enemy (`self.GetTransform` (`|GetArrayItem` _outactors (`KismetMathLibrary.RandomInteger` (`KismetArrayLibrary.Array_Length` _outactors)))) "Undefined" "OverrideRootScale" null null)
  (set `/Game/Interaction/Blueprints/Managers/Spawn/Spawn_Locations.CurrentSpawns` (+ (`/Game/Interaction/Blueprints/Managers/Spawn/Spawn_Locations.CurrentSpawns` _leastdistancespawns) 1.0) _leastdistancespawns))

(fn `SpawnVisable`
  (params (SpawnLocations :type "/Game/Interaction/Blueprints/Managers/Spawn/Spawn_Locations Object Reference") (PlayerLocation :type "Vector Structure"))
  (returns (IsNotVisable :type Boolean))
  (bind _outhit (`KismetSystemLibrary.SphereTraceSingle` :`Start` (`self.K2_GetActorLocation` SpawnLocations) :`End` PlayerLocation :`Radius` 0.5 :`TraceChannel` "TraceTypeQuery4" :`DrawDebugType` "ForOneFrame"))
  (return (and (!= (`.HitActor` (`GameplayStatics.BreakHitResult` _outhit)) "/Game/Interaction/Blueprints/Pawn/Player/Character_Pawn_FPS.Character_Pawn_FPS") (`/Game/Interaction/Blueprints/Managers/Spawn/Spawn_Locations.CanSpawn` SpawnLocations))))

(fn `UserConstructionScript`)