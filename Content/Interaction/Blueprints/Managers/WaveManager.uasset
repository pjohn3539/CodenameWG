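; Wave manager actor that runs point-budget enemy waves, spawning the spawn, enemy, aggro and group helper actors at BeginPlay.
; Each wave's composition meets per-type minimum percentages, then fills randomly up to maximum percentages.
; While active, Tick sends random groups to the spawn manager under an alive-points cap, refunded by EnemyDeath.
; A cleared wave raises both budgets, notifies the game mode, respawns the player, opens the exit and deactivates.
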(event `self.ReceiveBeginPlay`
  (bind _returnvalue (`|SpawnActorFromClass` "/Game/Interaction/Blueprints/Managers/Spawn_Manager.Spawn_Manager_C" (`KismetMathLibrary.MakeTransform` (0.0 0.0 0.0)) "Undefined" "OverrideRootScale" null null))
  (set `self.SpawnManager` _returnvalue)
  (bind _returnvalue_2 (`|SpawnActorFromClass` "/Game/Interaction/Blueprints/Managers/Enemy_Manager.Enemy_Manager_C" (`KismetMathLibrary.MakeTransform` (0.0 0.0 0.0)) "Undefined" "OverrideRootScale" null null))
  (bind _output_get (set `self.EnemyManager` _returnvalue_2))
  (set `/Game/Interaction/Blueprints/Managers/Spawn_Manager.EnemyManager` _output_get (`self.SpawnManager`))
  (`|SpawnActorFromClass` "/Game/Interaction/Blueprints/Managers/Aggro_Manager.Aggro_Manager_C" (`KismetMathLibrary.MakeTransform` (0.0 0.0 0.0)) "Undefined" "OverrideRootScale" null null)
  (bind _returnvalue_3 (`|SpawnActorFromClass` "/Game/Interaction/Blueprints/Managers/Enemy_Groups.Enemy_Groups_C" (`KismetMathLibrary.MakeTransform` (0.0 0.0 0.0)) "Undefined" "OverrideRootScale" null null))
  (`/Game/Interaction/Blueprints/Managers/Enemy_Groups.SetupEnemyGroups` _returnvalue_3 self)
  (set `self.MaxPoints` (`self.MaxPoints_Default`))
  (set `self.CurrentPoints` (`self.MaxPoints`))
  (`self.MinimumPercents`)
  (`self.CreateRemainingWave`)
  (`BlueprintMapLibrary.Map_Values` (`self.Wave`))
  (set `self.CurrentPoints` (`self.MaxPoints`)))

(event `self.ReceiveTick`
  (params (DeltaSeconds :type "Float (single-precision)"))
  (bind _currentpoints (`self.CurrentPoints`))
  (bind _wavenamesavailable (`self.WaveNamesAvailable`))
  (bind _currentpoints_2 (`self.CurrentPoints`))
  (bind _returnvalue (+ DeltaSeconds (`self.WaitCounter`)))
  (if (`self.Active`)
    (if (`self.Wait_Bool`)
      (if (>= _returnvalue (`self.Wait Time`))
        (set `self.WaitCounter` 0.0)
        (set `self.Wait_Bool` false)
        (`KismetSystemLibrary.PrintString` "New Wave Starting NOW!!!!!" true true (struct :`R` 1.0 :`B` 0.934104 :`A` 1.0) 30.0)
        (else
          (set `self.WaitCounter` _returnvalue)))
      (elif (and (>= (- (`KismetMathLibrary.Conv_IntToDouble` (/ (`KismetMathLibrary.FTrunc` (`self.MaxPointsAtOnce`)) (`self.Spawn-Groups`))) (`self.SpawnedPoints`)) (`KismetMathLibrary.Conv_IntToDouble` (/ (`KismetMathLibrary.FTrunc` (`self.Point_Threshold`)) (`self.Spawn-Groups`)))) (> (`self.CurrentPoints`) 0.0))
        (for _ (range (+ (`self.Spawn-Groups`) 1))
          (set `self.TempPoints` 0.0)
          (bind _output_get (set `self.WaveNamesAvailable` (`self.WaveNames`)))
          (for _array_element _output_get
            ;[1 1 1] Remove  enemies that aren't going to spawn in the wave
            (if (<= (`BlueprintMapLibrary.Map_Find` (`self.Wave`) _array_element) 0.0)
              (`KismetArrayLibrary.Array_RemoveItem` (`self.WaveNamesAvailable`) _array_element)))
          (set `self.GroupToSpawn` (`self.WaveReset`))
          (bind _asinteraction_game_mode_fps (cast `/Game/GameManagers/Interaction_GameMode_FPS` (`GameplayStatics.GetGameMode`)))
          (if (not (`/Game/GameManagers/Interaction_GameMode_FPS.IsGameOver` _asinteraction_game_mode_fps))
            (if (> (`KismetArrayLibrary.Array_Length` (`/Game/Interaction/Blueprints/Managers/Spawn_Manager.Players` (`self.SpawnManager`))) 0)
              (set `self.SubtractedSpawned` 0.0)
              (while (and (> (`KismetMathLibrary.Conv_IntToDouble` (/ (`KismetMathLibrary.FTrunc` (`self.MaxPointsAtOnce`)) (`self.Spawn-Groups`))) (`self.TempPoints`)) (> _currentpoints 0.0) (> _currentpoints (`self.TempPoints`)) (< (`self.SpawnedPoints`) (`self.MaxPointsAtOnce`)))
                (bind _output_get_2 (set `self.Random_Name` (`|GetArrayItem` _wavenamesavailable (`KismetMathLibrary.RandomInteger` (`KismetArrayLibrary.Array_Length` _wavenamesavailable)))))
                (bind _value (`BlueprintMapLibrary.Map_Find` (`self.WaveEnemyPoints`) _output_get_2))
                (if (and (>= _currentpoints_2 _value) (> (`BlueprintMapLibrary.Map_Find` (`self.Wave`) _output_get_2) 0.0) (>= (`KismetMathLibrary.Conv_IntToDouble` (/ (`KismetMathLibrary.FTrunc` (`self.MaxPointsAtOnce`)) (`self.Spawn-Groups`))) (+ (`self.TempPoints`) _value)))
                  (set `self.CurrentPoints` (- _currentpoints_2 _value))
                  (set `self.SpawnedPoints` (+ (`self.SpawnedPoints`) _value))
                  (set `self.TempPoints` (+ (`self.TempPoints`) _value))
                  (`BlueprintMapLibrary.Map_Add` (`self.Wave`) (`self.Random_Name`) (- (`BlueprintMapLibrary.Map_Find` (`self.Wave`) (`self.Random_Name`)) 1.0))
                  (`BlueprintMapLibrary.Map_Add` (`self.GroupToSpawn`) (`self.Random_Name`) (+ 1.0 (`BlueprintMapLibrary.Map_Find` (`self.GroupToSpawn`) (`self.Random_Name`))))
                  (`/Engine/EditorBlueprintResources/StandardMacros.IncrementInt` (`self.Amount_of_Enemies`))
                  (else
                    (`KismetArrayLibrary.Array_RemoveItem` (`self.WaveNamesAvailable`) (`self.Random_Name`))
                    (if (<= (`KismetArrayLibrary.Array_LastIndex` (`self.WaveNamesAvailable`)) -1)
                      (`KismetSystemLibrary.PrintString` "CRASH")))))
              (bind _values (`BlueprintMapLibrary.Map_Values` (`self.GroupToSpawn`)))
              (bind _spawned (`/Game/Interaction/Blueprints/Managers/Spawn_Manager.SpawnEnemies` (`self.SpawnManager`) (`self.EnemyClasses`) _values))
              (if _spawned
                (`KismetSystemLibrary.PrintString` (`KismetStringLibrary.Conv_DoubleToString` (`self.CurrentPoints`)) true true (struct :`R` 1.0 :`B` 0.934104 :`A` 1.0) 30.0)
                (`KismetSystemLibrary.PrintString` (`KismetStringLibrary.Conv_DoubleToString` (`self.SpawnedPoints`)) true true (struct :`R` 1.0 :`B` 0.934104 :`A` 1.0) 30.0)
                (else
                  (set `self.CurrentPoints` (+ (`self.CurrentPoints`) (`self.TempPoints`)))
                  (set `self.SpawnedPoints` (+ (`self.CurrentPoints`) (`self.TempPoints`))))))))
        (if true
          _)
        (elif (and (<= (`self.CurrentPoints`) 0.0) (<= (`self.SpawnedPoints`) 0.0))
          (bind _asinteraction_game_mode_fps_2 (cast `/Game/GameManagers/Interaction_GameMode_FPS` (`GameplayStatics.GetGameMode`)))
          (`/Game/GameManagers/Interaction_GameMode_FPS.WaveCompletedTextSequence` _asinteraction_game_mode_fps_2)
          (bind _output_get_3 (set `self.WaveCounter` (+ (`self.WaveCounter`) 1)))
          (`/Game/GameManagers/Interaction_GameMode_FPS.CallGameOver` _asinteraction_game_mode_fps_2 _output_get_3)
          (`KismetSystemLibrary.PrintString` "wave COMPLETED")
          (set `self.Wave` (`self.WaveReset`))
          (set `self.SpawnedPoints` 0.0)
          (set `self.MaxPoints` (+ (`self.MaxPoints`) (`self.MaxPointsIncrease`)))
          (set `self.CurrentPoints` (`self.MaxPoints`))
          (set `self.MaxPointsAtOnce` (+ (`self.MaxPointsAtOnce`) (`self.MaxPointsAtOnceIncrease`)))
          (`/Engine/EditorBlueprintResources/StandardMacros.IncrementInt` (`self.WaveNumber`)
            (:`  `
              (`KismetSystemLibrary.PrintString` "NEW WAVE" true true (struct :`R` 1.0 :`B` 0.934104 :`A` 1.0) 30.0)
              (`self.MinimumPercents`)
              (`self.CreateRemainingWave`)
              (set `self.CurrentPoints` (`self.MaxPoints`))
              (set `self.Amount_of_Enemies` 0)
              (set `self.WaitCounter` 0.0)
              (set `self.Wait_Bool` true)
              (set `self.Active` false)
              (bind _asinteraction_game_mode_fps_3 (cast `/Game/GameManagers/Interaction_GameMode_FPS` (`GameplayStatics.GetGameMode`)))
              (`/Game/GameManagers/Interaction_GameMode_FPS.RespawnPlayer` _asinteraction_game_mode_fps_3)
              (set `self.OpenExit` true))))))))

(event `Wait`
  (params (Second :type Integer)))

(event `SetWManager`
  (params (active :type Boolean))
  (if active
    (`KismetSystemLibrary.Delay` 3.0)
    (else
      (set `self.Active` false))))

(fn `CreateRemainingWave`
  (locals (RandomName :type String))
  (bind _randomname (`local.RandomName`))
  (bind _value (`BlueprintMapLibrary.Map_Find` (`self.WaveEnemyPoints`) _randomname))
  (bind _returnvalue (+ (`BlueprintMapLibrary.Map_Find` (`self.Wave`) _randomname) 1.0))
  (set `self.WaveNamesAvailable` (`self.WaveNames`))
  (while (> (`self.CurrentPoints`) 0.0)
    (set `local.RandomName` (`|GetArrayItem` (`self.WaveNamesAvailable`) (`KismetMathLibrary.RandomIntegerInRange` 0 (- (`KismetArrayLibrary.Array_Length` (`self.WaveNamesAvailable`)) 1))))
    (if (and (>= (`self.CurrentPoints`) _value) (<= (* 100.0 (/ (* _value _returnvalue) (`self.MaxPoints`))) (`BlueprintMapLibrary.Map_Find` (`self.WaveMaxPerct`) _randomname)))
      (`BlueprintMapLibrary.Map_Add` (`self.Wave`) _randomname _returnvalue)
      (set `self.CurrentPoints` (- (`self.CurrentPoints`) _value))
      (else
        (`KismetArrayLibrary.Array_RemoveItem` (`self.WaveNamesAvailable`) _randomname)))))

(fn `CreateWave`)

(fn `EnemyDeath`
  (params (DeadEnemy :type String))
  (bind _output_get (set `self.SpawnedPoints` (- (`self.SpawnedPoints`) (`BlueprintMapLibrary.Map_Find` (`self.WaveEnemyPoints`) DeadEnemy))))
  (`/Engine/EditorBlueprintResources/StandardMacros.DecrementInt` (`self.Amount_of_Enemies`)))

(fn `MinimumPercents`
  (for _array_element (`self.WaveNames`)
    (bind (_value _returnvalue) (`BlueprintMapLibrary.Map_Find` (`self.WaveMinPerct`) _array_element))
    (if _returnvalue
      (bind _value_2 (`BlueprintMapLibrary.Map_Find` (`self.WaveEnemyPoints`) _array_element))
      (bind _returnvalue_2 (`KismetMathLibrary.FTrunc` (/ (* (/ _value 100.0) (`self.MaxPoints`)) _value_2)))
      (`BlueprintMapLibrary.Map_Add` (`self.Wave`) _array_element (`KismetMathLibrary.Conv_IntToDouble` _returnvalue_2))
      (set `self.CurrentPoints` (- (`self.CurrentPoints`) (* _returnvalue_2 _value_2)))
      (else
        (`KismetSystemLibrary.PrintString` "A StringDoesn't match")))))

(fn `NextWave`
  (set `self.WaveNumber` (+ (`self.WaveNumber`) 1))
  (`KismetArrayLibrary.Array_Clear` (`self.Enemies`))
  (set `self.CurrentEnemyCount` 0)
  (set `self.WaveCapacity` (+ (`self.WaveCapacity`) 5))
  (set `self.EnemiesAliveCap` (+ (`self.EnemiesAliveCap`) 1)))

(fn `ResetWaveManager`
  (set `self.WaveCounter` 0)
  (set `self.Active` false)
  (set `self.WaveNumber` 1)
  (`/Game/Interaction/Blueprints/Managers/Enemy_Manager.ClearEnemies` (`self.EnemyManager`))
  (bind _output_get (set `self.MaxPoints` (`self.MaxPoints_Default`)))
  (set `self.CurrentPoints` _output_get)
  (set `self.MaxPointsAtOnce` (`self.MaxPointsAtOnce_Default`))
  (set `self.Wave` (`self.WaveReset`))
  (set `self.Amount_of_Enemies` 0)
  (set `self.WaitCounter` 0.0)
  (set `self.Wait_Bool` false)
  (`self.MinimumPercents`)
  (`self.CreateRemainingWave`)
  (`BlueprintMapLibrary.Map_Values` (`self.Wave`))
  (set `self.CurrentPoints` (`self.MaxPoints`)))

(fn `SetWaveManager`
  (params (Active :type Boolean))
  (if Active
    (set `self.Active` true)
    (`/Game/Interaction/Blueprints/Managers/Spawn_Manager.ResetSpawnManager` (`self.SpawnManager`))
    (else
      (set `self.Active` false))))

(fn `SubEnemyCount`
  (set `self.CurrentEnemyCount` (- (`self.CurrentEnemyCount`) 1))
  (if (and (>= (`KismetArrayLibrary.Array_Length` (`self.Enemies`)) (`self.WaveCapacity`)) (<= (`self.CurrentEnemyCount`) 0))
    (`self.NextWave`)))

(fn `UserConstructionScript`)