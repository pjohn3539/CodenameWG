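; Enemy group actor that holds a GroupSpawn map and totals the point cost of that group.
; On the first Tick, a DoOnce reads WaveEnemyPoints from the first WaveManager found in the level.
; It multiplies the two maps' values pairwise by index rather than key, so both need matching order.
; The summed TotalCost is printed on screen; the numbered GroupSpawn variables are unused.
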(event `self.ReceiveBeginPlay`)

(event `self.ReceiveTick`
  (params (DeltaSeconds :type "Float (single-precision)"))
  (bind _totalcost (`self.TotalCost`))
  (`/Engine/EditorBlueprintResources/StandardMacros.DoOnce` false
    (:`Completed`
      (bind _outactors (`GameplayStatics.GetAllActorsOfClass` "/Game/Interaction/Blueprints/Managers/WaveManager.WaveManager_C"))
      (set `self.EnemyPoints` (`/Game/Interaction/Blueprints/Managers/WaveManager.WaveEnemyPoints` (`|GetArrayItem` _outactors)))
      (bind _values (`BlueprintMapLibrary.Map_Values` (`self.EnemyPoints`)))
      (bind _values_2 (`BlueprintMapLibrary.Map_Values` (`self.GroupSpawn`)))
      (for (_array_element _array_index) _values_2
        (set `self.TotalCost` (+ (* _array_element (`|GetArrayItem` _values _array_index)) _totalcost)))
      (`KismetSystemLibrary.PrintString` (`KismetStringLibrary.Conv_DoubleToString` _totalcost) true true (struct :`G` 0.12266 :`B` 1.0 :`A` 1.0)))))

(fn `UserConstructionScript`)