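; Aggro manager that tracks how many enemy points target each FPS player, for balancing enemy targeting.
; It copies point values, classes and threshold from WaveManager, retrying on Tick while the class list is empty.
; AddEnemy and SubEnemy adjust player and total points, matching class index to map value order.
; Queries return the least-targeted player, flag swarmed players by share, and OutSideThreshold returns false when two players' shares are lopsided.
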(event `self.ReceiveBeginPlay`
  (bind _outactors (`GameplayStatics.GetAllActorsOfClass` "/Game/Interaction/Blueprints/Pawn/Player/Character_Pawn_FPS.Character_Pawn_FPS_C"))
  (for _array_element _outactors
    (`BlueprintMapLibrary.Map_Add` (`self.PlayersPoints`) _array_element)
    (`KismetSystemLibrary.PrintString` "Player set")
    (bind _outactors_2 (`GameplayStatics.GetAllActorsOfClass` "/Game/Interaction/Blueprints/Managers/WaveManager.WaveManager_C"))
    (for _array_element_2 _outactors_2
      (set `self.WaveEnemyPoints` (`/Game/Interaction/Blueprints/Managers/WaveManager.WaveEnemyPoints` _array_element_2))
      (set `self.EnemyClasses` (`/Game/Interaction/Blueprints/Managers/WaveManager.EnemyClasses` _array_element_2))
      (set `self.PointThreshold` (`/Game/Interaction/Blueprints/Managers/WaveManager.Point_Threshold` _array_element_2)))))

(event `self.ReceiveActorBeginOverlap`
  (params (OtherActor :type "Actor Object Reference")))

(event `self.ReceiveTick`
  (params (DeltaSeconds :type "Float (single-precision)"))
  (if (< (`KismetArrayLibrary.Array_LastIndex` (`self.EnemyClasses`)) 0)
    (bind _outactors (`GameplayStatics.GetAllActorsOfClass` "/Game/Interaction/Blueprints/Managers/WaveManager.WaveManager_C"))
    (for _array_element _outactors
      (set `self.WaveEnemyPoints` (`/Game/Interaction/Blueprints/Managers/WaveManager.WaveEnemyPoints` _array_element))
      (set `self.EnemyClasses` (`/Game/Interaction/Blueprints/Managers/WaveManager.EnemyClasses` _array_element))
      (set `self.PointThreshold` (`/Game/Interaction/Blueprints/Managers/WaveManager.Point_Threshold` _array_element))
      (`KismetSystemLibrary.PrintString` "GOT IT!!!" true true (struct :`G` 0.66 :`B` 1.0 :`A` 1.0) 50.0)
      (bind _outactors_2 (`GameplayStatics.GetAllActorsOfClass` "/Game/Interaction/Blueprints/Pawn/Player/Character_Pawn_FPS.Character_Pawn_FPS_C"))
      (for _array_element_2 _outactors_2
        (`BlueprintMapLibrary.Map_Add` (`self.PlayersPoints`) _array_element_2)))))

(fn `AddEnemy`
  (params (EnemyClass :type "Actor Class Reference") (Player :type "/Game/Interaction/Blueprints/Pawn/Player/Character_Pawn_FPS Object Reference"))
  (bind _playerspoints (`self.PlayersPoints`))
  (bind _returnvalue (`KismetArrayLibrary.Array_Find` (`self.EnemyClasses`) EnemyClass))
  (bind (_value _returnvalue_2) (`BlueprintMapLibrary.Map_Find` _playerspoints Player))
  (bind _values (`BlueprintMapLibrary.Map_Values` (`self.WaveEnemyPoints`)))
  (bind _keys (`BlueprintMapLibrary.Map_Keys` (`self.WaveEnemyPoints`)))
  (`KismetSystemLibrary.PrintString` (`|GetArrayItem` _keys _returnvalue) true true (struct :`R` 1.0 :`B` 0.686432 :`A` 1.0))
  (if (and (> _returnvalue -1) _returnvalue_2)
    (bind _output (`|GetArrayItem` _values _returnvalue))
    (`BlueprintMapLibrary.Map_Add` _playerspoints Player (+ _value _output))
    (set `self.Current Points` (+ _output (`self.Current Points`)))))

(fn `GetLeastAggro`
  (params (Player1 :type "/Game/Interaction/Blueprints/Pawn/Player/Character_Pawn_FPS Object Reference") (Player2 :type "/Game/Interaction/Blueprints/Pawn/Player/Character_Pawn_FPS Object Reference"))
  (returns (PlayerToAggro :type "/Game/Interaction/Blueprints/Pawn/Player/Character_Pawn_FPS Object Reference"))
  (bind _playerspoints (`self.PlayersPoints`))
  (if (<= (`BlueprintMapLibrary.Map_Find` _playerspoints Player1) (`BlueprintMapLibrary.Map_Find` _playerspoints Player2))
    (return Player1)
    (else
      (return Player2))))

(fn `OutSideThreshold`
  (params (Player1 :type "/Game/Interaction/Blueprints/Pawn/Player/Character_Pawn_FPS Object Reference") (Player2 :type "/Game/Interaction/Blueprints/Pawn/Player/Character_Pawn_FPS Object Reference"))
  (returns (NotOutsidePerctage :type Boolean))
  (bind _playerspoints (`self.PlayersPoints`))
  (bind _returnvalue (/ (`BlueprintMapLibrary.Map_Find` _playerspoints Player2) (`self.Current Points`)))
  (bind _returnvalue_2 (/ (`BlueprintMapLibrary.Map_Find` _playerspoints Player1) (`self.Current Points`)))
  (if (and (>= _returnvalue_2 (`self.MaxPercent`)) (<= _returnvalue (`self.MinPercent`)))
    _
    (elif (and (<= _returnvalue_2 (`self.MinPercent`)) (>= _returnvalue (`self.MaxPercent`)))
      _
      (else
        (return true))))
  (return false))

(fn `PlayerOverTargeted`
  (params (TargetPlayer :type "/Game/Interaction/Blueprints/Pawn/Player/Character_Pawn_FPS Object Reference"))
  (returns (isSwarmed :type Boolean))
  (bind _current_points (`self.Current Points`))
  (if (and (>= (/ (`BlueprintMapLibrary.Map_Find` (`self.PlayersPoints`) TargetPlayer) _current_points) (`self.SwarmPercent`)) (> _current_points (`self.PointThreshold`)))
    (return true)
    (else
      (return false))))

(fn `SubEnemy`
  (params (EnemyClass :type "Actor Class Reference") (Player :type "/Game/Interaction/Blueprints/Pawn/Player/Character_Pawn_FPS Object Reference"))
  (bind _playerspoints (`self.PlayersPoints`))
  (bind _returnvalue (`KismetArrayLibrary.Array_Find` (`self.EnemyClasses`) EnemyClass))
  (bind (_value _returnvalue_2) (`BlueprintMapLibrary.Map_Find` _playerspoints Player))
  (bind _values (`BlueprintMapLibrary.Map_Values` (`self.WaveEnemyPoints`)))
  (bind _keys (`BlueprintMapLibrary.Map_Keys` (`self.WaveEnemyPoints`)))
  (`KismetSystemLibrary.PrintString` (`|GetArrayItem` _keys _returnvalue) true true (struct :`R` 1.0 :`B` 0.686432 :`A` 1.0))
  (if (and (> _returnvalue -1) _returnvalue_2)
    (bind _output (`|GetArrayItem` _values _returnvalue))
    (`BlueprintMapLibrary.Map_Add` _playerspoints Player (- _value _output))
    (set `self.Current Points` (- (`self.Current Points`) _output))))

(fn `UserConstructionScript`)