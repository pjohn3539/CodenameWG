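; Base melee weapon Blueprint that tracks a charged attack while the action button is held.
; Pressing resets the timer, Tick accumulates it up to MaxChargeTime, and releasing calls SetColliders to switch hit colliders on.
; ResetObject clears the charge and turns colliders off.
; SetColliders is an empty stub here, and BeginPlay sets the maximum attack index.
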(event `self.ReceiveBeginPlay`
  (`parent.ReceiveBeginPlay`)
  (set `self.WeaponAttackIndexMax` 4))

(event `self.ReceiveTick`
  (params (DeltaSeconds :type "Float (single-precision)"))
  (bind _returnvalue (+ DeltaSeconds (`self.Timer`)))
  (`parent.ReceiveTick` DeltaSeconds)
  (if (`self.Pressed`)
    (if (< _returnvalue (`self.MaxChargeTime`))
      (set `self.Timer` _returnvalue)
      (else
        (set `self.Timer` (`self.MaxChargeTime`))))))

(event `/Game/Interaction/Blueprints/Weapon/Base_Interactive_Object_Class.ActionButtonPressed`
  (set `self.Pressed` true)
  (set `self.Timer` 0.0))

(event `/Game/Interaction/Blueprints/Weapon/Base_Interactive_Object_Class.ActionButtonReleased`
  (if (`self.Pressed`)
    (set `self.Pressed` false)
    (`self.SetColliders` true)))

(event `/Game/Interaction/Blueprints/Weapon/Base_Interactive_Object_Class.ResetObject`
  (set `self.Timer` 0.0)
  (set `self.Pressed` false)
  (`self.SetColliders` false))

(fn `SetColliders`
  (params (Active :type Boolean)))

(fn `UserConstructionScript`
  (`parent.UserConstructionScript`))