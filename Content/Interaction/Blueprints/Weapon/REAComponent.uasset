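; REAComponent is a weapon data component that holds crosshair spread radius and recoil response values for different movement stances.
; Two initializers store default, walk, crouch and crouch-walk values for radius and recoil multiplier, plus the radius increment and maximum crosshair recoil, and reset current values to defaults.
; Getters and setters expose the current radius and recoil multiplier, with no update logic in the component itself.
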(fn `GetMovementCurrent`
  (returns (Current :type "Float (double-precision)"))
  (return (`self.Radius_Size_Current`)))

(fn `GetShotResponseCurrent`
  (returns (Current :type "Float (double-precision)"))
  (return (`self.RecoilMultiplier (pixels)_Current`)))

(fn `InitializeREA_Movement`
  (params (movementChanges :type Boolean) (movementDef :type "Float (double-precision)") (movementIncrement :type "Float (double-precision)") (movementWalk :type "Float (double-precision)") (movementCrouch :type "Float (double-precision)") (movement_cWalk :type "Float (double-precision)"))
  (set `self.Changes` movementChanges)
  (bind _output_get (set `self.Radius_Size_Default` movementDef))
  (set `self.Radius_Size_Current` _output_get)
  (set `self.Radius_Size_Increment` movementIncrement)
  (set `self.Radius_Size_Walk` movementWalk)
  (set `self.Radius_Size_Crouch` movementCrouch)
  (set `self.Radius_Size_Crouch_Walk` movement_cWalk))

(fn `InitializeREA_Shot_Response`
  (params (shotDef :type "Float (double-precision)") (shotWalk :type "Float (double-precision)") (shotCrouch :type "Float (double-precision)") (shot_cWalk :type "Float (double-precision)") (Crosshair_Recoil_Max :type "Float (double-precision)"))
  (bind _output_get (set `self.RecoilMultiplier (pixels)_Default` shotDef))
  (set `self.RecoilMultiplier (pixels)_Current` _output_get)
  (set `self.RecoilMultiplier (pixels)_Walk` shotWalk)
  (set `self.RecoilMultiplier (pixels)_Crouch` shotCrouch)
  (set `self.RecoilMultiplier (pixels)_CrouchWalk` shot_cWalk)
  (set `self.Crosshair_Element_Recoil_Max` Crosshair_Recoil_Max))

(fn `SetMovementCurrent`
  (params (Current :type "Float (double-precision)"))
  (set `self.Radius_Size_Current` Current))

(fn `SetShotResponseCurrent`
  (params (Current :type "Float (double-precision)"))
  (set `self.RecoilMultiplier (pixels)_Current` Current))