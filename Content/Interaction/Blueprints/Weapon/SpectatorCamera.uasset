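; SpectatorCamera is a camera rig that orbits on a spring arm.
; While Active is set, Tick advances the arm's world yaw by DeltaSeconds times SpeedModifier and holds pitch and roll at zero.
; ResetCamera sets the spring arm's world transform with no transform supplied, so it returns to the default value rather than a stored starting pose.
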(event `self.ReceiveTick`
  (params (DeltaSeconds :type "Float (single-precision)"))
  (bind _springarm (`self.SpringArm`))
  (bind (_returnvalue_roll _returnvalue_pitch _returnvalue_yaw) (`KismetMathLibrary.BreakRotator` (`SceneComponent.K2_GetComponentRotation` _springarm)))
  (if (`self.Active`)
    (`SceneComponent.K2_SetWorldRotation` _springarm (`KismetMathLibrary.MakeRotator` 0.0 0.0 (+ _returnvalue_yaw (* DeltaSeconds (`self.SpeedModifier`)))) false false)))

(fn `ResetCamera`
  (`SceneComponent.K2_SetWorldTransform` (`self.SpringArm`) (`KismetMathLibrary.MakeTransform` (0.0 0.0 0.0)) false false))

(fn `UserConstructionScript`)