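; Inventory component for the FPS player pawn, holding primary and secondary weapons, a temporary object, grenade counts and quest-item state.
; PickUpItem fills slots from a pickup or spawned StartingWeapon, physically throws displaced objects forward, then calls the player's AddWeapon.
; AddAmmo clamps to storage capacity, returning overflow to weapon pickups, while AddGrenade caps each type.
; Key, card, valve, password and rifle-ammo pickup macros remain, but their event-graph dispatch never runs.
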(event `PickUpItem`
  (params (Name :type String) (PickUpWeapon :type "/Game/Interaction/Maps/Blueprints/BP_PickupItem_Weapon Object Reference") (FromStart :type Boolean :default false) (WeaponIndex :type Integer) (Instantiate :type Boolean) (PkupWeapon :type "/Game/Interaction/Blueprints/Weapon/Base_Interactive_Object_Class Object Reference"))
  (`/Engine/EditorBlueprintResources/StandardMacros.IsValid` PkupWeapon
    (:`Is Valid`
      (bind _asbase_weapon_class (cast `/Game/Interaction/Blueprints/Weapon/Base_Weapon_Class` PkupWeapon))
      (if (not (`/Game/Interaction/Blueprints/Weapon/Base_Weapon_Class.IsTemporary` _asbase_weapon_class))
        (bind (_newweapon _replace) (`self.SetNonTempWeapon` _asbase_weapon_class FromStart))
        (`/Game/Interaction/Blueprints/Pawn/Player/Character_Pawn_FPS.AddWeapon` (`self.Player`) _newweapon _replace)
        (else
          (bind _objectadded (`self.SetTempObject` _asbase_weapon_class))
          (`/Game/Interaction/Blueprints/Pawn/Player/Character_Pawn_FPS.AddWeapon` (`self.Player`) _objectadded false))))
    (:`Is Not Valid`
      (bind _returnvalue (`|SpawnActorFromClass` (`self.StartingWeapon`) (`Actor.GetTransform` (`self.GetOwner`)) "Undefined" "OverrideRootScale" null null))
      (bind (_newweapon_2 _replace_2) (`self.SetNonTempWeapon` _returnvalue FromStart))
      (`/Game/Interaction/Blueprints/Pawn/Player/Character_Pawn_FPS.AddWeapon` (`self.Player`) _newweapon_2 _replace_2))))

(event `Interp`
  (bind _arammocurrent (`self.ARAmmoCurrent`))
  (bind _asweapon_ammo_class (cast `/Game/Interaction/Blueprints/Weapon/Weapon_Ammo_Class` (`/Game/Interaction/Blueprints/Pawn/Player/Character_Pawn_FPS.CWeapon` (`self.Player`))))
  (set `/Game/Interaction/Blueprints/Weapon/Weapon_Ammo_Class.Ammo_Supply` (`KismetMathLibrary.FTrunc` (`KismetMathLibrary.FClamp` (`KismetMathLibrary.Lerp` _arammocurrent (+ _arammocurrent (`self.ARAmmo+`)) (+ (/ (`self.ForTimer`) 0.5) 0.07)) 0.0 (`KismetMathLibrary.Conv_IntToDouble` (`/Game/Interaction/Blueprints/Weapon/Weapon_Ammo_Class.Ammo_MaxStorageSize` _asweapon_ammo_class)))) _asweapon_ammo_class)
  (set `self.ForTimer` (+ (`self.ForTimer`) 0.01)))

(fn `AddAmmo`
  (params (Amount :type Integer) (WeaponAddedTo :type "/Game/Interaction/Blueprints/Weapon/Weapon_Ammo_Class Object Reference") (FromWeaponPickup :type Boolean) (WeaponPickup :type "/Game/Interaction/Blueprints/Weapon/Weapon_Ammo_Class Object Reference"))
  (locals (WeaponAddAmmo :type "/Game/Interaction/Blueprints/Weapon/Weapon_Ammo_Class Object Reference") (AddedAmmo :type "Float (double-precision)") (CurrentAmmo :type "Float (double-precision)") (IsPrim :type Boolean) (FromWP :type Boolean) (PrevCurrent :type "Float (double-precision)") (AmmoLeft :type Integer) (WP :type "/Game/Interaction/Blueprints/Weapon/Weapon_Ammo_Class Object Reference"))
  (set `local.WP` WeaponPickup)
  (bind _output_get (set `local.FromWP` FromWeaponPickup))
  (if _output_get
    (set `local.AddedAmmo` (`KismetMathLibrary.Conv_IntToDouble` (`/Game/Interaction/Blueprints/Weapon/Weapon_Ammo_Class.Ammo_Supply` (`local.WP`))))
    (else
      (set `local.AddedAmmo` (`KismetMathLibrary.Conv_IntToDouble` Amount))))
  (set `local.WeaponAddAmmo` WeaponAddedTo)
  (`|ExecutionSequence`
    (:`then_0`
      (bind _output_get_2 (set `local.CurrentAmmo` (`KismetMathLibrary.Conv_IntToDouble` (`/Game/Interaction/Blueprints/Weapon/Weapon_Ammo_Class.Ammo_Supply` (`local.WeaponAddAmmo`)))))
      (set `local.PrevCurrent` _output_get_2)
      (bind _output_get_3 (set `self.PrimaryAmmoCurrent` (`KismetMathLibrary.Conv_IntToDouble` (`KismetMathLibrary.FTrunc` (`KismetMathLibrary.FClamp` (+ (`local.CurrentAmmo`) (`local.AddedAmmo`)) 0.0 (`KismetMathLibrary.Conv_IntToDouble` (`/Game/Interaction/Blueprints/Weapon/Weapon_Ammo_Class.Ammo_MaxStorageSize` (`local.WeaponAddAmmo`))))))))
      (set `/Game/Interaction/Blueprints/Weapon/Weapon_Ammo_Class.Ammo_Supply` (`KismetMathLibrary.FTrunc` _output_get_3) (`local.WeaponAddAmmo`))
      (if (> (`local.AddedAmmo`) 0.0)
        (`GameplayStatics.PlaySound2D` (`self.PickupAmmoSound`))))
    (:`then_1`
      (if (`local.FromWP`)
        (if (>= (+ (`local.PrevCurrent`) (`local.AddedAmmo`)) (`KismetMathLibrary.Conv_IntToDouble` (`/Game/Interaction/Blueprints/Weapon/Weapon_Ammo_Class.Ammo_MaxStorageSize` (`local.WeaponAddAmmo`))))
          (set `/Game/Interaction/Blueprints/Weapon/Weapon_Ammo_Class.Ammo_Supply` (mod (`KismetMathLibrary.FTrunc` (+ (`local.PrevCurrent`) (`local.AddedAmmo`))) (`/Game/Interaction/Blueprints/Weapon/Weapon_Ammo_Class.Ammo_MaxStorageSize` (`local.WeaponAddAmmo`))) (`local.WP`))
          (else
            (set `/Game/Interaction/Blueprints/Weapon/Weapon_Ammo_Class.Ammo_Supply` 0 (`local.WP`))))))))

(fn `AddGrenade`
  (params (Type :type "/Game/Interaction/Blueprints/Weapon/Grenades/GrenadeType Enum" :default "NewEnumerator0"))
  (returns (Destroy :type Boolean))
  (locals (DestroyPickup :type Boolean))
  (switch `/Game/Interaction/Blueprints/Weapon/Grenades/GrenadeType` Type
    (:`NewEnumerator0`
      (if (< (`self.BasicGrenadeAmount`) (`self.MaxGrenadeAmount`))
        (set `self.BasicGrenadeAmount` (+ (`self.BasicGrenadeAmount`) 1))
        (set `local.DestroyPickup` true)
        (else
          (set `local.DestroyPickup` false))))
    (:`NewEnumerator1`
      (if (< (`self.StickyGrenadeAmount`) (`self.MaxGrenadeAmount`))
        (set `self.StickyGrenadeAmount` (+ (`self.StickyGrenadeAmount`) 1))
        (set `local.DestroyPickup` true)
        (else
          (set `local.DestroyPickup` false))))
    (:`NewEnumerator2`
      (if (< (`self.FlameGrenadeAmount`) (`self.MaxGrenadeAmount`))
        (set `self.FlameGrenadeAmount` (+ (`self.FlameGrenadeAmount`) 1))
        (set `local.DestroyPickup` true)
        (else
          (set `local.DestroyPickup` false)))))
  (return (`local.DestroyPickup`)))

(fn `DisableObjectColliders`
  (params (Object :type "/Game/Interaction/Blueprints/Weapon/Base_Interactive_Object_Class Object Reference"))
  (bind _physics (`/Game/Interaction/Blueprints/Weapon/Base_Interactive_Object_Class.Physics` Object))
  (`PrimitiveComponent.SetSimulatePhysics` _physics false)
  (`PrimitiveComponent.SetCollisionEnabled` _physics "NoCollision")
  (`PrimitiveComponent.SetCollisionEnabled` (`/Game/Interaction/Blueprints/Weapon/Base_Interactive_Object_Class.Trigger` Object) "NoCollision"))

(fn `DropObject`
  (params (Object :type "/Game/Interaction/Blueprints/Weapon/Base_Interactive_Object_Class Object Reference"))
  (bind _physics (`/Game/Interaction/Blueprints/Weapon/Base_Interactive_Object_Class.Physics` Object))
  (`SceneComponent.K2_DetachFromComponent` (`/Game/Interaction/Blueprints/Weapon/Base_Interactive_Object_Class.Physics` Object) "KeepRelative" "KeepRelative" "KeepRelative" false)
  (`Actor.K2_SetActorLocation` Object (`SceneComponent.K2_GetComponentLocation` (`/Game/Interaction/Blueprints/Pawn/Player/Character_Pawn_FPS.DropLocation` (`self.Player`))) false false)
  (set `/Game/Interaction/Blueprints/Weapon/Base_Interactive_Object_Class.IsEquip` false Object)
  (set `/Game/Interaction/Blueprints/Weapon/Base_Interactive_Object_Class.Player` null Object)
  (`PrimitiveComponent.SetSimulatePhysics` _physics true)
  (`PrimitiveComponent.SetCollisionEnabled` _physics "PhysicsOnly")
  (`PrimitiveComponent.SetCollisionEnabled` (`/Game/Interaction/Blueprints/Weapon/Base_Interactive_Object_Class.Trigger` Object) "QueryOnly")
  (`PrimitiveComponent.AddImpulse` _physics (* (`Actor.GetActorForwardVector` (`self.Player`)) 350.0) "None" true)
  (if (== Object (`self.TempObject`))
    (set `self.TempObject` null)))

(fn `SetNonTempWeapon`
  (params (Weapon :type "/Game/Interaction/Blueprints/Weapon/Base_Weapon_Class Object Reference") (FromStart :type Boolean))
  (returns (NewWeapon :type "/Game/Interaction/Blueprints/Weapon/Base_Weapon_Class Object Reference") (Replace :type Boolean))
  (locals (CallReplace :type Boolean))
  (bind _ascharacter_pawn_fps (`self.Player`))
  (bind _ascharacter_pawn_fps_2 (`self.Player`))
  (bind _ascharacter_pawn_fps_3 (`self.Player`))
  (if (not (not (`KismetSystemLibrary.IsValid` (`self.TempObject`))))
    (`self.DropObject` (`self.TempObject`)))
  (set `/Game/Interaction/Blueprints/Weapon/Base_Interactive_Object_Class.Player` _ascharacter_pawn_fps_3 Weapon)
  (if FromStart
    (set `self.PrimaryWeapon` Weapon :!label _label)
    (set `/Game/Interaction/Blueprints/Pawn/Player/Character_Pawn_FPS.CurrentWeaponIndex` 1 _ascharacter_pawn_fps_2)
    (`self.DisableObjectColliders` (`self.PrimaryWeapon`))
    (elif (== (`/Game/Interaction/Blueprints/Pawn/Player/Character_Pawn_FPS.CurrentWeaponIndex` _ascharacter_pawn_fps_3) 1)
      (`/Engine/EditorBlueprintResources/StandardMacros.IsValid` (`self.PrimaryWeapon`)
        (:`Is Valid`
          (`/Engine/EditorBlueprintResources/StandardMacros.IsValid` (`self.SecondaryWeapon`)
            (:`Is Valid`
              (set `local.CallReplace` true)
              (`self.DropObject` (`self.PrimaryWeapon`))
              (goto _label))
            (:`Is Not Valid`
              (set `self.SecondaryWeapon` Weapon)
              (set `/Game/Interaction/Blueprints/Pawn/Player/Character_Pawn_FPS.CurrentWeaponIndex` 2 _ascharacter_pawn_fps_2)
              (`self.DisableObjectColliders` (`self.SecondaryWeapon`)))))
        (:`Is Not Valid`
          (goto _label)))
      (else
        (`/Engine/EditorBlueprintResources/StandardMacros.IsValid` (`self.SecondaryWeapon`)
          (:`Is Valid`
            (`/Engine/EditorBlueprintResources/StandardMacros.IsValid` (`self.PrimaryWeapon`)
              (:`Is Valid`
                (set `local.CallReplace` true)
                (`self.DropObject` (`self.SecondaryWeapon`))
                (set `self.SecondaryWeapon` Weapon :!label _label_2)
                (set `/Game/Interaction/Blueprints/Pawn/Player/Character_Pawn_FPS.CurrentWeaponIndex` 2 _ascharacter_pawn_fps)
                (`self.DisableObjectColliders` (`self.SecondaryWeapon`)))
              (:`Is Not Valid`
                (set `self.PrimaryWeapon` Weapon)
                (set `/Game/Interaction/Blueprints/Pawn/Player/Character_Pawn_FPS.CurrentWeaponIndex` 1 _ascharacter_pawn_fps)
                (`self.DisableObjectColliders` (`self.PrimaryWeapon`)))))
          (:`Is Not Valid`
            (goto _label_2))))))
  (return Weapon (`local.CallReplace`)))

(fn `SetTempObject`
  (params (NewObject :type "/Game/Interaction/Blueprints/Weapon/Base_Interactive_Object_Class Object Reference") (FromStart :type Boolean))
  (returns (ObjectAdded :type "/Game/Interaction/Blueprints/Weapon/Base_Interactive_Object_Class Object Reference") (Replace :type Boolean))
  (locals (CallReplace :type Boolean) (NewTempObject :type "/Game/Interaction/Blueprints/Weapon/Base_Interactive_Object_Class Object Reference"))
  (bind _output_get (set `local.NewTempObject` NewObject))
  (set `/Game/Interaction/Blueprints/Weapon/Base_Interactive_Object_Class.Player` (`self.Player`) _output_get)
  (`/Engine/EditorBlueprintResources/StandardMacros.IsValid` (`self.TempObject`)
    (:`Is Valid`
      (`self.DropObject` (`self.TempObject`)))
    (:`Is Not Valid`
      _))
  (bind _output_get_2 (set `self.TempObject` (`local.NewTempObject`)))
  (`self.DisableObjectColliders` _output_get_2)
  (return _output_get_2 false))