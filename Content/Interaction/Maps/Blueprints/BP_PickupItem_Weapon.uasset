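; Weapon pickup actor that builds on a parent pickup class and represents a weapon item in the world.
; On BeginPlay it runs the parent logic, points the Mesh reference at its skeletal mesh and sets a very short pickup delay.
; CheckSuppy destroys the actor when its ammo amount is depleted, though nothing in this file calls it.
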(event `self.ReceiveBeginPlay`
  (`parent.ReceiveBeginPlay`)
  (set `self.Mesh` (`self.ItemSkeletalMesh`))
  (set `self.DelayItemPickup` 0.01))

(fn `CheckSuppy`
  (if (<= (`self.AmmoAmount`) 0)
    (`self.K2_DestroyActor`)))

(fn `UserConstructionScript`
  (`parent.UserConstructionScript`))