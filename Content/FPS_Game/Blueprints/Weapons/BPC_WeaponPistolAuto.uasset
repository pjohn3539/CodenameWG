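; Automatic pistol weapon Blueprint for the FPS game, a child class that adds mesh animations to inherited weapon behavior.
; WeaponFire calls the parent, then plays a non-looping animation on the first- and third-person meshes if ammo remains and the player is not reloading.
; ReloadWeapon calls the parent, then animates both meshes when MagCheck passes.
; Reload and the construction script only forward to the parent.
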(event `self.WeaponFire`
  (`parent.WeaponFire`)
  (if (> (`self.AmmoCurrent`) 0)
    (if (not (`/Game/FPS_Game/Blueprints/BP_CharacterBase.isReloading` (`self.PlayerCast`)))
      ;[1 1 1] Add your weapon animations here
      (`SkeletalMeshComponent.PlayAnimation` (`self.Weapon_Mesh_FPP`) null false)
      (`SkeletalMeshComponent.PlayAnimation` (`self.Weapon_Mesh_TPP`) null false))))

(event `self.ReloadWeapon`
  (`parent.ReloadWeapon`)
  (bind _canreload (`self.MagCheck`))
  (if _canreload
    ;[1 1 1] Add your weapon animations here
    (`SkeletalMeshComponent.PlayAnimation` (`self.Weapon_Mesh_FPP`) null false)
    (`SkeletalMeshComponent.PlayAnimation` (`self.Weapon_Mesh_TPP`) null false)))

(event `self.Reload`
  (`parent.Reload`))

(fn `UserConstructionScript`
  (`parent.UserConstructionScript`))