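; Base weapon Blueprint for player firearms, highlighted through custom depth on overlap and added to the inventory on interaction.
; Looping-timer or single WeaponFire calls consume ammo, then branch into projectile or hitscan shots, supporting first/third person and ADS spread.
; Camera traces drive hitscan damage with headshot multipliers and aim muzzle-spawned projectiles, with optional camera spawning.
; An empty magazine triggers reload, which waits for the montage before drawing on reserve ammo.
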(event `self.Sphere.OnComponentBeginOverlap`
  (params (OverlappedComponent :type "PrimitiveComponent Object Reference") (OtherActor :type "Actor Object Reference") (OtherComp :type "PrimitiveComponent Object Reference") (OtherBodyIndex :type Integer) (bFromSweep :type Boolean) (SweepResult :type "HitResult Structure (by ref)"))
  (bind _sphere (`self.Sphere`))
  ;[1 1 1] Draw the outline for the weapon on overlap with the character, disable collision for the overlap sphere when the weapon is picked up (to prevent the outline from staying visible)
  (cast `/Game/FPS_Game/Blueprints/BP_CharacterBase` OtherActor)
  (`PrimitiveComponent.SetRenderCustomDepth` (`self.Weapon_Mesh_FPP`) true)
  (`PrimitiveComponent.SetRenderCustomDepth` (`self.Weapon_Mesh_TPP`) true)
  (`PrimitiveComponent.SetCollisionResponseToChannel` _sphere "ECC_Camera" "ECR_Block")
  (`PrimitiveComponent.SetCollisionResponseToChannel` _sphere "ECC_Visibility" "ECR_Block"))

(event `self.Sphere.OnComponentEndOverlap`
  (params (OverlappedComponent :type "PrimitiveComponent Object Reference") (OtherActor :type "Actor Object Reference") (OtherComp :type "PrimitiveComponent Object Reference") (OtherBodyIndex :type Integer))
  (bind _sphere (`self.Sphere`))
  ;[1 1 1] Draw the outline for the weapon on overlap with the character, disable collision for the overlap sphere when the weapon is picked up (to prevent the outline from staying visible)
  (cast `/Game/FPS_Game/Blueprints/BP_CharacterBase` OtherActor)
  (`PrimitiveComponent.SetRenderCustomDepth` (`self.Weapon_Mesh_FPP`) false)
  (`PrimitiveComponent.SetRenderCustomDepth` (`self.Weapon_Mesh_TPP`) false)
  (`PrimitiveComponent.SetCollisionResponseToChannel` _sphere "ECC_Camera" "ECR_Ignore")
  (`PrimitiveComponent.SetCollisionResponseToChannel` _sphere "ECC_Visibility" "ECR_Ignore"))

(event `self.ReceiveBeginPlay`
  ;[1 1 1] Begin Play
  (bind _asbp_character_base (cast `/Game/FPS_Game/Blueprints/BP_CharacterBase` (`GameplayStatics.GetPlayerCharacter` 0)))
  (set `self.PlayerCast` _asbp_character_base)
  (`|ExecutionSequence`
    (:`then_0`
      (bind _returnvalue (`|CreateWidget` "/Game/FPS_Game/UI/W_Scope.W_Scope_C"))
      (bind _output_get (set `self.Scope` _returnvalue))
      (`UserWidget.AddToViewport` _output_get -15)
      (`Widget.SetVisibility` _output_get "Hidden")
      (set `self.SpawnedWeapon` self))
    (:`then_1`
      (`Image.SetBrushFromTexture` (`/Game/FPS_Game/UI/W_Scope.Scope_Texture_IMG` (`self.Scope`)) (`self.CustomScopeOverlayTexture`) false))))

(event `/Game/FPS_Game/Blueprints/System/BPI_Interact.BPI_Interaction`
  (bind _playercast (`self.PlayerCast`))
  ;[1 1 1] Add to player inventory
  (set `/Game/FPS_Game/Blueprints/BP_CharacterBase.isReloading` false _playercast)
  (bind _indexoftheaddedweapon (`/Game/FPS_Game/Blueprints/BP_CharacterBase.AddWeapon` _playercast (`self.SpawnedWeapon`)))
  ;;[1 1 1] Prevents the weapon from showing up in player hands before the swapping animation has finished
  (`/Game/FPS_Game/Blueprints/BP_CharacterBase.PlaySwappingMontage` _playercast)
  (`self.SetActorHiddenInGame` true)
  (`KismetSystemLibrary.Delay` (`/Game/FPS_Game/Blueprints/BP_CharacterBase.SwappingWeaponDelay` _playercast))
  (`self.SetActorHiddenInGame` false)
  (`/Game/FPS_Game/Blueprints/BP_CharacterBase.EquipWeapon` _playercast _indexoftheaddedweapon)
  ;[1 1 1] Draw the outline for the weapon on overlap with the character, disable collision for the overlap sphere when the weapon is picked up (to prevent the outline from staying visible)
  (`PrimitiveComponent.SetCollisionEnabled` (`self.Sphere`) "NoCollision"))

(event `AutoFireStart`
  ;[1 1 1] Automatic firing
  (`KismetSystemLibrary.K2_SetTimer` null "WeaponFire" (`self.FireRate`) true))

(event `AutoFireStop`
  ;[1 1 1] Automatic firing
  (`KismetSystemLibrary.K2_ClearTimer` null "WeaponFire"))

(event `WeaponFire`
  (bind _projectilespawnfrommuzzlefpp (`self.ProjectileSpawnFromMuzzleFPP`))
  (bind _playercast (`self.PlayerCast`))
  (bind _playercast_2 (`self.PlayerCast`))
  (bind _playercast_3 (`self.PlayerCast`))
  (bind _playercast_4 (`self.PlayerCast`))
  (bind _gunoffset (`/Game/FPS_Game/Blueprints/BP_CharacterBase.GunOffset` _playercast))
  (bind _firstpersoncamera (`/Game/FPS_Game/Blueprints/BP_CharacterBase.FirstPersonCamera` (`self.PlayerCast`)))
  (bind _thirdpersoncamera (`/Game/FPS_Game/Blueprints/BP_CharacterBase.ThirdPersonCamera` (`self.PlayerCast`)))
  (bind _gunoffset_2 (`/Game/FPS_Game/Blueprints/BP_CharacterBase.GunOffset` _playercast_2))
  (if (not (`/Game/FPS_Game/Blueprints/BP_CharacterBase.isReloading` _playercast_3))
    (if (`/Game/FPS_Game/Blueprints/BP_CharacterBase.isADS` _playercast_3)
      (`/Game/FPS_Game/Blueprints/BP_CharacterBase.ADS_Speed` _playercast_4)
      (else
        (`/Game/FPS_Game/Blueprints/BP_CharacterBase.WalkSpeed` _playercast_4)))
    (if (`/Game/FPS_Game/Blueprints/BP_CharacterBase.GamepadVibration` _playercast_4)
      (`GameplayStatics.SpawnForceFeedbackAttached` (`self.GamepadVibrationForceFeedback`) (`self.DefaultSceneRoot`)))
    (if (`self.InfiniteAmmo`)
      (`GameplayStatics.PlaySoundAtLocation` (`self.FiringSound`) (`self.K2_GetActorLocation`) :!label _label) ; Play firing sound
      (switch `/Game/FPS_Game/Blueprints/Weapons/Base/E_WeaponType` (`self.WeaponType`)
        (:`NewEnumerator1`
          (if (`/Game/FPS_Game/Blueprints/BP_CharacterBase.isFPP` (`self.PlayerCast`))
            (for _ (range (+ (`self.AdditionalBulletsToFire`) 1))
              (bind _outhit (`self.LineTraceWeapon`))
              (bind (_bblockinghit _binitialoverlap _time _location _impactpoint) (`GameplayStatics.BreakHitResult` _outhit))
              (`|SpawnActorFromClass` (`self.ProjectileToFire`) (select `bool` (`self.ProjectileSpawnsFromCamera`) :`false` (`self.ProjectileSpawnTransform_GunBarrel` _projectilespawnfrommuzzlefpp _gunoffset (`KismetMathLibrary.MakeRotFromX` (- (select `bool` _bblockinghit :`false` (+ (`SceneComponent.K2_GetComponentLocation` _firstpersoncamera) (* (`SceneComponent.GetForwardVector` _firstpersoncamera) 100000.0)) :`true` _impactpoint) (`SceneComponent.K2_GetComponentLocation` _projectilespawnfrommuzzlefpp)))) :`true` (`self.ProjectileSpawnTransform` (`/Game/FPS_Game/Blueprints/BP_CharacterBase.ProjectileSpawn` _playercast) _gunoffset (`/Game/FPS_Game/Blueprints/BP_CharacterBase.FirstPersonCamera` _playercast))) "AlwaysSpawn" "OverrideRootScale" null (`self.Damage`) null)
              (`self.MuzzleFlashEffect` (`self.Weapon_Mesh_FPP`) (`self.MuzzlePoint`))
              ;[1 1 1] AnimMontages for the character and camera shake
              (`self.Play_FireAnimMontages` :!label _label_2)
              (`PlayerCameraManager.PlayCameraShake` :`self` (`GameplayStatics.GetPlayerCameraManager` 0) :`ShakeClass` (`self.CameraShake`) :`Scale` (`self.CameraShakeScale`)))
            (else
              (for _ (range (+ (`self.AdditionalBulletsToFire`) 1))
                (bind _outhit_2 (`self.LineTraceWeapon`))
                (bind (_bblockinghit_2 _binitialoverlap_2 _time_2 _location_2 _impactpoint_2) (`GameplayStatics.BreakHitResult` _outhit_2))
                (`|SpawnActorFromClass` (`self.ProjectileToFire`) (select `bool` (`self.ProjectileSpawnsFromCamera`) :`false` (`self.ProjectileSpawnTransform_GunBarrel` (`self.ProjectileSpawnFromMuzzleTPP`) _gunoffset_2 (`KismetMathLibrary.MakeRotFromX` (- (select `bool` _bblockinghit_2 :`false` (+ (`SceneComponent.K2_GetComponentLocation` _thirdpersoncamera) (* (`SceneComponent.GetForwardVector` _thirdpersoncamera) 100000.0)) :`true` _impactpoint_2) (`SceneComponent.K2_GetComponentLocation` (`self.ProjectileSpawnFromMuzzleTPP`))))) :`true` (`self.ProjectileSpawnTransform` (`/Game/FPS_Game/Blueprints/BP_CharacterBase.ProjectileSpawnTPP` _playercast_2) _gunoffset_2 (`/Game/FPS_Game/Blueprints/BP_CharacterBase.ThirdPersonCamera` _playercast_2))) "AlwaysSpawn" "OverrideRootScale" null (`self.Damage`) null)
                (`self.MuzzleFlashEffect` (`self.Weapon_Mesh_TPP`) (`self.MuzzlePoint`))
                (goto _label_2)))))
        (:`NewEnumerator2`
          (for _ (range (+ (`self.AdditionalBulletsToFire`) 1))
            (bind _outhit_3 (`self.LineTraceWeapon`))
            (bind (_bblockinghit_3 _binitialoverlap_3 _time_3 _location_3 _impactpoint_3 _normal _impactnormal _physmat _hitactor _hitcomponent _hitbonename) (`GameplayStatics.BreakHitResult` _outhit_3))
            (`GameplayStatics.ApplyDamage` _hitactor (select `bool` (== _hitbonename "head") :`false` (`self.Damage`) :`true` (* (`self.Damage`) (`self.Damage_CriticalHitMultiplierForHitscan`))))
            (`/Engine/EditorBlueprintResources/StandardMacros.IsValid` _hitactor
              (:`Is Valid`
                (if (`self.ActorHasTag` _hitactor "Enemy")
                  (`GameplayStatics.SpawnEmitterAtLocation` null _impactpoint_3 (`KismetMathLibrary.RandomRotator` false))
                  (else
                    (`GameplayStatics.SpawnEmitterAtLocation` null _impactpoint_3 (`KismetMathLibrary.RandomRotator` false) :!label _label_3))))
              (:`Is Not Valid`
                (goto _label_3)))
            (`GameplayStatics.SpawnDecalAttached` null (15.0 15.0 15.0) _hitcomponent "None" _impactpoint_3 (`KismetMathLibrary.ComposeRotators` (`KismetMathLibrary.MakeRotator` (`KismetMathLibrary.RandomFloatInRange` 0.0 360.0)) (`KismetMathLibrary.MakeRotFromX` _normal)) "KeepWorldPosition")
            (`GameplayStatics.PlaySoundAtLocation` null _impactpoint_3)
            (`self.Play_FireAnimMontages`)
            (`PlayerCameraManager.PlayCameraShake` :`self` (`GameplayStatics.GetPlayerCameraManager` 0) :`ShakeClass` (`self.CameraShake`) :`Scale` (`self.CameraShakeScale`))
            (if (`/Game/FPS_Game/Blueprints/BP_CharacterBase.isFPP` (`self.PlayerCast`))
              (`self.MuzzleFlashEffect` (`self.Weapon_Mesh_FPP`) (`self.MuzzlePoint`))
              (else
                (`self.MuzzleFlashEffect` (`self.Weapon_Mesh_TPP`) (`self.MuzzlePoint`)))))))
      (else
        (bind _hasammo (`self.AmmoCheck`))
        (if _hasammo
          (goto _label)
          (else
            (`self.ReloadWeapon`)
            (`GameplayStatics.PlaySoundAtLocation` (`self.NoAmmoSound`) (`self.K2_GetActorLocation`)) ; Play no ammo sound
          ))))))

(event `ReloadWeapon`
  (bind _playercast (`self.PlayerCast`))
  (`self.AutoFireStop`)
  (bind _canreload (`self.MagCheck`))
  (if _canreload
    (if (not (`/Game/FPS_Game/Blueprints/BP_CharacterBase.isReloading` _playercast))
      (set `/Game/FPS_Game/Blueprints/BP_CharacterBase.isReloading` true _playercast)
      (bind _animmontageduration (`self.Play_ReloadAnimMontages`))
      (`KismetSystemLibrary.Delay` _animmontageduration)
      (`self.Reload`)
      (set `/Game/FPS_Game/Blueprints/BP_CharacterBase.isReloading` false _playercast))
    (elif (not (== (`self.AmmoCurrent`) (`self.AmmoMax`)))
      (`GameplayStatics.PlaySoundAtLocation` (`self.NoAmmoSound`) (`self.K2_GetActorLocation`)) ; Play no ammo sound
    )))

(fn `AddAmmo`
  (params (AmmoToAdd :type Integer))
  (set `self.AmmoInReserve` (`KismetMathLibrary.Clamp` (+ (`self.AmmoInReserve`) AmmoToAdd) (`self.Zero`) (`self.AmmoInReserve_Max`))))

(fn `AmmoCheck`
  (returns (HasAmmo :type Boolean))
  (`/Engine/EditorBlueprintResources/StandardMacros.CompareInt` (`self.AmmoCurrent`) (`self.Zero`)
    (:`>`
      (set `self.AmmoCurrent` (- (`self.AmmoCurrent`) 1))
      (return true))
    (:`==`
      _)
    (:`<`
      _))
  (set `self.AmmoCurrent` (`self.Zero`))
  (return false))

(fn `LineTraceWeapon`
  (returns (OutHit :type "HitResult Structure") (ReturnValue :type Boolean))
  (bind _playercast (`self.PlayerCast`))
  (bind _firstpersoncamera (`/Game/FPS_Game/Blueprints/BP_CharacterBase.FirstPersonCamera` _playercast))
  (bind _ut_inventory (`/Game/FPS_Game/Blueprints/BP_CharacterBase.UT_Inventory` _playercast))
  (bind _thirdpersoncamera (`/Game/FPS_Game/Blueprints/BP_CharacterBase.ThirdPersonCamera` _playercast))
  (bind _returnvalue (`SceneComponent.K2_GetComponentLocation` _firstpersoncamera))
  (bind _returnvalue_2 (`SceneComponent.K2_GetComponentLocation` _thirdpersoncamera))
  (bind _returnvalue_3 (+ _returnvalue_2 (* (`SceneComponent.GetForwardVector` _thirdpersoncamera) 100000.0)))
  (bind _returnvalue_4 (+ _returnvalue (* (`SceneComponent.GetForwardVector` _firstpersoncamera) 10000.0)))
  (`/Engine/EditorBlueprintResources/StandardMacros.IsValid` _playercast
    (:`Is Valid`
      (if (`/Game/FPS_Game/Blueprints/BP_CharacterBase.isFPP` _playercast)
        ;[1 1 1] First Person Camera LineTrace
        (if (`/Game/FPS_Game/Blueprints/BP_CharacterBase.isADS` (`self.PlayerCast`))
          ;;[1 1 1] FPS - aiming down sights
          (bind (_outhit _returnvalue_5) (`KismetSystemLibrary.LineTraceSingle` _returnvalue (`self.SprayForLineTraceWeapon` _returnvalue_4 (`self.BulletSpreadADS`)) "TraceTypeQuery1" false _ut_inventory))
          (return _outhit _returnvalue_5)
          (else
            (bind (_outhit_2 _returnvalue_6) (`KismetSystemLibrary.LineTraceSingle` _returnvalue (`self.SprayForLineTraceWeapon` _returnvalue_4 (`self.BulletSpread`)) "TraceTypeQuery1" false _ut_inventory))
            (return _outhit_2 _returnvalue_6)))
        (else
          ;[1 1 1] Third Person Camera LineTrace
          (if (`/Game/FPS_Game/Blueprints/BP_CharacterBase.isADS` (`self.PlayerCast`))
            ;;[1 1 1] TPS - aiming down sights
            (bind (_outhit_3 _returnvalue_7) (`KismetSystemLibrary.LineTraceSingle` _returnvalue_2 (`self.SprayForLineTraceWeapon` _returnvalue_3 (`self.BulletSpreadADS`)) "TraceTypeQuery1" false _ut_inventory))
            (return _outhit_3 _returnvalue_7)
            (else
              (bind (_outhit_4 _returnvalue_8) (`KismetSystemLibrary.LineTraceSingle` _returnvalue_2 (`self.SprayForLineTraceWeapon` _returnvalue_3 (`self.BulletSpread`)) "TraceTypeQuery1" false _ut_inventory))
              (return _outhit_4 _returnvalue_8))))))))

(fn `MagCheck`
  (returns (CanReload :type Boolean))
  (return (and (>= (`self.AmmoInReserve`) 1) (< (`self.AmmoCurrent`) (`self.AmmoMax`)))))

(fn `Reload`
  (bind _zero (`self.Zero`))
  (bind _output_get (set `self.AmmoNeeded` (- (`self.AmmoMax`) (`self.AmmoCurrent`))))
  (set `self.AmmoCurrent` (`self.AmmoMax`))
  (bind _returnvalue (- (`self.AmmoInReserve`) _output_get))
  (`/Engine/EditorBlueprintResources/StandardMacros.CompareInt` _returnvalue _zero
    (:`>`
      (set `self.AmmoInReserve` _returnvalue))
    (:`==`
      (set `self.AmmoInReserve` _zero :!label _label))
    (:`<`
      (goto _label))))

(fn `UserConstructionScript`)