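; Explosive red barrel that damages nearby actors and flings patrol AI when it blows up.
; Any damage activates its particle effect and explodes it after a two-second delay; striking a patrol AI at high speed detonates it immediately.
; The blast enlarges the overlap Sphere, plays sound and particles, then destroys the barrel.
; Sphere overlaps damage anything except wheeled vehicles and launch patrol AI with randomized velocity in positive X/Y.
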(event `Boom`
  (bind _returnvalue (`self.K2_GetActorLocation`))
  (bind _sphere (`self.Sphere`))
  (bind _particlesystem (`self.ParticleSystem`))
  (`SphereComponent.SetSphereRadius` _sphere 400.0 true :!label _label)
  (`SceneComponent.SetHiddenInGame` _sphere false false)
  (`/Engine/EditorBlueprintResources/StandardMacros.IsValid` _particlesystem
    (:`Is Valid`
      (`ActorComponent.Deactivate` _particlesystem))
    (:`Is Not Valid`
      _))
  (`GameplayStatics.PlaySoundAtLocation` "/Game/FPS_Game/Sounds/SFX/Explosion_Cue.Explosion_Cue" _returnvalue)
  (`GameplayStatics.SpawnEmitterAtLocation` "/Game/FPS_Game/Particles/Explosion_Big/P_Explosion_Big.P_Explosion_Big" _returnvalue)
  (`self.K2_DestroyActor`))

(event `self.ReceiveAnyDamage`
  (params (Damage :type "Float (single-precision)") (DamageType :type "DamageType Object Reference") (InstigatedBy :type "Controller Object Reference") (DamageCauser :type "Actor Object Reference"))
  (`ActorComponent.Activate` (`self.ParticleSystem`) false)
  (`KismetSystemLibrary.Delay` 2.0)
  (goto _label))

(event `self.Sphere.OnComponentBeginOverlap`
  (params (OverlappedComponent :type "PrimitiveComponent Object Reference") (OtherActor :type "Actor Object Reference") (OtherComp :type "PrimitiveComponent Object Reference") (OtherBodyIndex :type Integer) (bFromSweep :type Boolean) (SweepResult :type "HitResult Structure (by ref)"))
  (bind _returnvalue (`KismetMathLibrary.RandomFloatInRange` 400.0 500.0))
  (cast `WheeledVehicle` OtherActor
    (:`CastFailed`
      (`GameplayStatics.ApplyDamage` OtherActor 0.2 null self)
      (bind _asbp_ai_char_patrol (cast `/Game/FPS_Game/Blueprints/AI/Patrol/BP_AI_CharPatrol` OtherActor))
      (`Character.LaunchCharacter` _asbp_ai_char_patrol (`KismetMathLibrary.MakeVector` _returnvalue _returnvalue 50.0) true true))))

(event `self.ReceiveBeginPlay`)

(event `self.StaticMesh.OnComponentHit`
  (params (HitComponent :type "PrimitiveComponent Object Reference") (OtherActor :type "Actor Object Reference") (OtherComp :type "PrimitiveComponent Object Reference") (NormalImpulse :type "Vector Structure") (Hit :type "HitResult Structure (by ref)"))
  (cast `/Game/FPS_Game/Blueprints/AI/Patrol/BP_AI_CharPatrol` OtherActor)
  (if (or (> (`KismetMathLibrary.Abs` (.x (`self.GetVelocity`))) 1500.0) (> (`KismetMathLibrary.Abs` (.y (`self.GetVelocity`))) 1500.0) (> (`KismetMathLibrary.Abs` (.z (`self.GetVelocity`))) 1500.0))
    (`self.Boom`)))

(fn `UserConstructionScript`)