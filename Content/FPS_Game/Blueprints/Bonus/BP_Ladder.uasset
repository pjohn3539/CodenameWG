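; BP_Ladder is a climbable ladder that puts any BP_CharacterBase into climbing while it overlaps the actor.
; The construction script builds rung meshes procedurally, spaced by Offset over the height between LadderBottom and LadderTop, with shadows disabled.
; It also scales and raises a Box component to match that height.
; Begin and end overlap events call StartClimb and StopClimb on the character, which handles the climbing itself.
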(event `self.ReceiveActorBeginOverlap`
  (params (OtherActor :type "Actor Object Reference"))
  (bind _asbp_character_base (cast `/Game/FPS_Game/Blueprints/BP_CharacterBase` OtherActor))
  (`/Game/FPS_Game/Blueprints/BP_CharacterBase.StartClimb` _asbp_character_base))

(event `self.ReceiveActorEndOverlap`
  (params (OtherActor :type "Actor Object Reference"))
  (bind _asbp_character_base (cast `/Game/FPS_Game/Blueprints/BP_CharacterBase` OtherActor))
  (`/Game/FPS_Game/Blueprints/BP_CharacterBase.StopClimb` _asbp_character_base))

(fn `UserConstructionScript`
  (bind _offset (`self.Offset`))
  (bind (_returnvalue_x _returnvalue_y _returnvalue_z) (`KismetMathLibrary.BreakVector` (- (`self.LadderTop`) (`self.LadderBottom`))))
  (bind _returnvalue (/ _returnvalue_z 60.0))
  (for _index (range (+ (`KismetMathLibrary.FTrunc` (/ _returnvalue_z _offset)) 1))
    (bind _returnvalue_2 (`AddComponent|NODE_AddStaticMeshComponent-0` :`RelativeTransform` (`KismetMathLibrary.MakeTransform` (`KismetMathLibrary.MakeVector` 0.0 0.0 (* _index _offset)) (struct) (0.5 0.1 0.05))))
    (`PrimitiveComponent.SetCastShadow` _returnvalue_2 false)
    (`PrimitiveComponent.SetMaterial` _returnvalue_2 0 "/Game/FPS_Game/Weapons/FPProjectile/FirstPersonProjectileMaterial.FirstPersonProjectileMaterial"))
  (`SceneComponent.SetRelativeScale3D` (`self.Box`) (`KismetMathLibrary.MakeVector` 1.0 1.0 _returnvalue))
  (`SceneComponent.K2_AddRelativeLocation` (`self.Box`) (`KismetMathLibrary.MakeVector` 0.0 0.0 (* _returnvalue 30.0)) false false))