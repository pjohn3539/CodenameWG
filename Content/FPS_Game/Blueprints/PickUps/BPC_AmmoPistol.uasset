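; Pistol ammo pickup that refills a character's pistol reserve ammo on overlap.
; When a BP_CharacterBase with a valid equipped weapon overlaps it, it scans the inventory for BPC_WeaponPistol or BPC_WeaponPistolAuto by exact class.
; Matches below max reserve receive a fixed amount through AddAmmo and the pickup destroys itself, while full ones only print a max-ammo message.
; The loop has no break, so several matching pistols can each gain ammo.
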(event `self.ReceiveActorBeginOverlap`
  (params (OtherActor :type "Actor Object Reference"))
  (bind _asbp_character_base (cast `/Game/FPS_Game/Blueprints/BP_CharacterBase` OtherActor))
  (`/Engine/EditorBlueprintResources/StandardMacros.IsValid` (`/Game/FPS_Game/Blueprints/BP_CharacterBase.EquippedWeapon` _asbp_character_base)
    (:`Is Valid`
      (for _array_element (`/Game/FPS_Game/Blueprints/BP_CharacterBase.UT_Inventory` _asbp_character_base)
        (if (or (== (`GameplayStatics.GetObjectClass` _array_element) "/Game/FPS_Game/Blueprints/Weapons/BPC_WeaponPistol.BPC_WeaponPistol_C") (== (`GameplayStatics.GetObjectClass` _array_element) "/Game/FPS_Game/Blueprints/Weapons/BPC_WeaponPistolAuto.BPC_WeaponPistolAuto_C"))
          (if (== (`/Game/FPS_Game/Blueprints/Weapons/Base/BP_WeaponBase.AmmoInReserve_Max` _array_element) (`/Game/FPS_Game/Blueprints/Weapons/Base/BP_WeaponBase.AmmoInReserve` _array_element))
            (`KismetSystemLibrary.PrintString` "MAX  AMMO")
            (else
              (`/Game/FPS_Game/Blueprints/Weapons/Base/BP_WeaponBase.AddAmmo` _array_element 10)
              (`KismetSystemLibrary.PrintString` "AMMO  ADDED")
              (`self.K2_DestroyActor`))))))))

(fn `UserConstructionScript`
  (`parent.UserConstructionScript`))