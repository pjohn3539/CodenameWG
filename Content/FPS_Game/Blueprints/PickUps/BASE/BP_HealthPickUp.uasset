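; BP_HealthPickUp is a pickup that heals an overlapping BP_CharacterBase character by HealthToAdd.
; On overlap it compares the character's current health to its max, calling HealthHeal and destroying itself only when health is below max.
; At or above max it just prints a message and stays in the world.
; The construction script gives the actor a random relative rotation without roll.
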(event `self.ReceiveActorBeginOverlap`
  (params (OtherActor :type "Actor Object Reference"))
  (bind _asbp_character_base (cast `/Game/FPS_Game/Blueprints/BP_CharacterBase` OtherActor))
  (`/Engine/EditorBlueprintResources/StandardMacros.CompareFloat` (`/Game/FPS_Game/Blueprints/BP_CharacterBase.HealthCurrent` _asbp_character_base) (`/Game/FPS_Game/Blueprints/BP_CharacterBase.HealthMax` _asbp_character_base)
    (:`>`
      (`KismetSystemLibrary.PrintString` "MAX  HEALTH" :!label _label))
    (:`==`
      (goto _label))
    (:`<`
      (`/Game/FPS_Game/Blueprints/BP_CharacterBase.HealthHeal` _asbp_character_base (`self.HealthToAdd`))
      (`KismetSystemLibrary.PrintString` "HEALTH  ADDED")
      (`self.K2_DestroyActor`))))

(fn `UserConstructionScript`
  (`self.K2_SetActorRelativeRotation` (`KismetMathLibrary.RandomRotator` false)))